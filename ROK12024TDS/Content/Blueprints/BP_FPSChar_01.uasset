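; Player shooter character with an assault rifle, health and a HUD widget, moved along its capsule's axes.
; While alive, it turns toward the direction of mouse movement, interpolating control yaw once mouse speed exceeds a dead zone.
; Each fire press starts muzzle effects and sound, then runs one debug-drawn line trace from the muzzle socket to apply damage.
; Damage reduces clamped health, sets death at zero and always stops firing effects.
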(event `self.ReceiveBeginPlay`
  (bind _returnvalue (`|CreateWidget` "/Game/UI/PlayerHUD.PlayerHUD_C" null self))
  (`UserWidget.AddToViewport` _returnvalue 0))

(event `InputAction|Fire`
  (params (Key :type "Key Structure"))
  (:`Pressed`
    (if (`self.Is Alive `)
      (`self.StartFired`)
      (`self.weapon trace`)))
  (:`Released`
    (`self.StopFired`)
    (if (`self.Is Alive `)
      (`GameplayStatics.SpawnSound2D` "/Game/Sounds/Weapon_AssaultRifle/Stereo/AssaultRifle_ShotEnd02_Stereo.AssaultRifle_ShotEnd02_Stereo" 1.0 1.0 0.0 null))))

(event `self.ReceiveTick`
  (params (DeltaSeconds :type "Float (single-precision)"))
  (if (`self.Is Alive `)
    (`self.RotateCharacter`)))

(event `self.ReceiveAnyDamage`
  (params (Damage :type "Float (single-precision)") (DamageType :type "DamageType Object Reference") (InstigatedBy :type "Controller Object Reference") (DamageCauser :type "Actor Object Reference"))
  (bind _output_get (set `self.Health` (`KismetMathLibrary.FClamp` (- (`self.Health`) Damage) 0.0 100.0)))
  (set `self.dead` (== _output_get 0.0))
  (if true
    (`self.StopFired`)))

(event `InputAxis|MoveForwadBack`
  (params (AxisValue :type "Float (single-precision)"))
  (`self.AddMovementInput` (`SceneComponent.GetForwardVector` (`self.CapsuleComponent`)) AxisValue))

(event `InputAxis|MoveLeftRight`
  (params (AxisValue :type "Float (single-precision)"))
  (`self.AddMovementInput` (`SceneComponent.GetRightVector` (`self.CapsuleComponent`)) AxisValue))

(fn `GetEndLoczation LT`
  (returns (ReturnValue :type "Vector Structure"))
  (return (+ (`self.GetStartLocationLT`) (* (`KismetMathLibrary.GetForwardVector` (`self.GetControlRotation`)) (`self.Weapon R`)))))

(fn `GetStartLocationLT`
  (returns (ReturnValue :type "Vector Structure"))
  (return (`SceneComponent.GetSocketLocation` (`self.SkeletalMesh`) "P_AssaultRifle_MF")))

(fn `Is Alive `
  (returns (ReturnValue :type Boolean))
  (return (not (`self.dead`))))

(fn `IsMouseDeadZone`
  (returns (ReturnValue :type Boolean))
  (return (> (`KismetMathLibrary.VSize2D` (`self.MouseVelocity`)) (`self.DeadZone`))))

(fn `MouseVelocity`
  (returns (ReturnValue :type "Vector2D Structure"))
  (bind (_deltax _deltay) (`PlayerController.GetInputMouseDelta` (`GameplayStatics.GetPlayerController` 0)))
  (return (/ (`KismetMathLibrary.MakeVector2D` _deltax _deltay) (`GameplayStatics.GetWorldDeltaSeconds`))))

(fn `RotateCharacter`
  (bind _returnvalue (`GameplayStatics.GetPlayerController` 0))
  (bind (_returnvalue_x _returnvalue_y) (`KismetMathLibrary.BreakVector2D` (`self.MouseVelocity`)))
  (if (`self.IsMouseDeadZone`)
    (`Controller.SetControlRotation` _returnvalue (`KismetMathLibrary.RInterpTo` (`Controller.GetControlRotation` _returnvalue) (`KismetMathLibrary.MakeRotator` 0.0 0.0 (`KismetMathLibrary.DegAtan2` _returnvalue_x _returnvalue_y)) (`GameplayStatics.GetWorldDeltaSeconds`) (`self.Interp Speed`)))))

(fn `StartFired`
  (`ActorComponent.Activate` (`self.P_AssaultRifle_MF`) false)
  (bind _returnvalue (`GameplayStatics.SpawnSound2D` "/Game/Sounds/Weapon_AssaultRifle/Stereo/NewSoundCue.NewSoundCue" 1.0 1.0 0.0 null))
  (set `self.FIRESOUND` _returnvalue))

(fn `StopFired`
  (bind _firesound (`self.FIRESOUND`))
  (`ActorComponent.Deactivate` (`self.P_AssaultRifle_MF`))
  (`/Engine/EditorBlueprintResources/StandardMacros.IsValid` _firesound
    (:`Is Valid`
      (`AudioComponent.Stop` _firesound))))

(fn `UserConstructionScript`)

(fn `weapon trace`
  (bind _outhit (`KismetSystemLibrary.LineTraceSingle` :`Start` (`self.GetStartLocationLT`) :`End` (`self.GetEndLoczation LT`) :`TraceChannel` "TraceTypeQuery1" :`DrawDebugType` "ForDuration"))
  (`GameplayStatics.ApplyDamage` (`.HitActor` (`GameplayStatics.BreakHitResult` _outhit)) (`self.DamagePreHit`)))